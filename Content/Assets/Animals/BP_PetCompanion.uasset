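; BP_PetCompanion is a pet pawn that starts following the player once they first enter its trigger.
; That first overlap removes the Cylinder component and calls FollowPlayer, which runs AI MoveTo toward the player character with an acceptance radius.
; Each successful move re-calls FollowPlayer after a short delay, forming the follow loop.
; A failed move has no handler, so following stops there.
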(event `self.Trigger.OnComponentBeginOverlap`
  (params (OverlappedComponent :type "PrimitiveComponent Object Reference") (OtherActor :type "Actor Object Reference") (OtherComp :type "PrimitiveComponent Object Reference") (OtherBodyIndex :type Integer) (bFromSweep :type Boolean) (SweepResult :type "HitResult Structure (by ref)"))
  ; Check To Follow Character
  (if (== OtherActor (`GameplayStatics.GetPlayerPawn` 0))
    (`/Engine/EditorBlueprintResources/StandardMacros.DoOnce` false
      (:`Completed`
        (`ActorComponent.K2_DestroyComponent` (`self.Cylinder`))
        (`self.Follow Player`)))))

(event `Follow Player`
  ; Follow Character
  (`|AIMoveTo` self (0.0 0.0 0.0) (`GameplayStatics.GetPlayerCharacter` 0) 150.0
    (:`OnSuccess`
      (`KismetSystemLibrary.Delay` 1.0)
      (`self.Follow Player`))))

(fn `UserConstructionScript`)