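; Inspection actor that lets the player examine an item's mesh and materials, supplied through InspectInfo, in a WB_InspectView widget.
; Inspect swaps input from player to actor; IA_Inspect returns it, restores the interaction prompt and destroys the actor.
; Left-drag rotates the mesh, the wheel moves the SceneCapture camera within clamped zoom limits, and right-click resets both.
; Middle-click toggles full and detailed views through forward and reversed widget animations.
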(event `/Game/Interaction/BPI_Interaction.Inspect`
  (params (InspectInfo :type "/Game/Interaction/Inspect/S_InspectInfo Structure"))
  (bind (_itemmesh _itemmaterials) (break `/Game/Interaction/Inspect/S_InspectInfo` InspectInfo))
  (bind _returnvalue (`GameplayStatics.GetPlayerController` 0))
  (`self.CreateInspectView` InspectInfo)
  (`StaticMeshComponent.SetStaticMesh` (`self.InspectMesh`) _itemmesh)
  (for (_array_element _array_index) _itemmaterials
    (`PrimitiveComponent.SetMaterial` (`self.InspectMesh`) _array_index _array_element)
    (`self.DisableInput` (`/Game/Interaction/BP_UniversalLibrary.GetMyPlayer`) _returnvalue)
    (`self.EnableInput` _returnvalue)))

(event `EnhancedInput|/Game/Input/Actions/IA_Inspect`
  (params (ActionValue :type Boolean) (ElapsedSeconds :type "Float (double-precision)") (TriggeredSeconds :type "Float (double-precision)") (InputAction :type "InputAction Object Reference" :default "/Game/Input/Actions/IA_Inspect.IA_Inspect"))
  (bind _returnvalue (`GameplayStatics.GetPlayerController` 0))
  (:`Started`
    (`self.DisableInput` _returnvalue)
    (`self.EnableInput` (`/Game/Interaction/BP_UniversalLibrary.GetMyPlayer`) _returnvalue)
    (bind _wb_inspectview (`self.WB_InspectView`)
      (:`then`
        (`Widget.RemoveFromParent` _wb_inspectview)
        (`UserWidget.AddToViewport` (`/Game/Interaction/BPC_Intercation.WB_InteractMessage` (`self.GetComponentByClass` (`/Game/Interaction/BP_UniversalLibrary.GetMyPlayer`) "/Game/Interaction/BPC_Intercation.BPC_Intercation_C")) 0)
        (`self.K2_DestroyActor`))
      (:`else`))))

(event `InputAxisKey|MouseX`
  (params (AxisValue :type "Float (single-precision)"))
  ;[0 0 0 0.5] Horizontal Movement
  (if (`self.ShouldRotate`)
    (`SceneComponent.K2_SetWorldRotation` (`self.InspectMesh`) (`KismetMathLibrary.ComposeRotators` (`SceneComponent.K2_GetComponentRotation` (`self.InspectMesh`)) (`KismetMathLibrary.MakeRotator` 0.0 0.0 (* AxisValue -4.0))) false false)))

(event `Key|LeftMouseButton`
  (params (Key :type "Key Structure"))
  ;[0 0 0 0.5] Allows Rotation
  (:`Pressed`
    (set `self.ShouldRotate` true))
  (:`Released`
    (set `self.ShouldRotate` false)))

(event `Key|RightMouseButton`
  (params (Key :type "Key Structure"))
  ;[0 0 0 0.5] Resets Inspect
  (:`Pressed`
    (`SceneComponent.K2_SetRelativeLocation` (`self.SceneCaptureComponent2D`) (-250.0 0.0 0.0) false false)
    (`SceneComponent.K2_SetWorldRotation` :`self` (`self.InspectMesh`))))

(event `InputAxisKey|MouseY`
  (params (AxisValue :type "Float (single-precision)"))
  ;[0 0 0 0.5] Vertical Movement
  (if (`self.ShouldRotate`)
    (`SceneComponent.K2_SetWorldRotation` (`self.InspectMesh`) (`KismetMathLibrary.ComposeRotators` (`SceneComponent.K2_GetComponentRotation` (`self.InspectMesh`)) (`KismetMathLibrary.MakeRotator` 0.0 (* AxisValue -4.0))) false false)))

(event `Key|MiddleMouseButton`
  (params (Key :type "Key Structure"))
  ;[0 0 0 0.5] Switches Between full and detailed view
  (:`Pressed`
    (if (not (`self.ZoomIn`))
      (set `self.ZoomIn` true)
      (`self.ZoomInFade`)
      (else
        (set `self.ZoomIn` false)
        (`self.ZoomOutFade`)))))

(event `Key|MouseScrollUp`
  (params (Key :type "Key Structure"))
  (bind (_relativelocation_x _relativelocation_y _relativelocation_z) (`KismetMathLibrary.BreakVector` (`SceneComponent.RelativeLocation` (`self.SceneCaptureComponent2D`))))
  ;[0 0 0 0.5] Zoom In
  (:`Pressed`
    (`SceneComponent.K2_SetRelativeLocation` (`self.SceneCaptureComponent2D`) (`KismetMathLibrary.MakeVector` (`KismetMathLibrary.FClamp` (+ _relativelocation_x 20.0) -400.0 -160.0) _relativelocation_y _relativelocation_z) false false)))

(event `Key|MouseScrollDown`
  (params (Key :type "Key Structure"))
  (bind (_relativelocation_x _relativelocation_y _relativelocation_z) (`KismetMathLibrary.BreakVector` (`SceneComponent.RelativeLocation` (`self.SceneCaptureComponent2D`))))
  ;[0 0 0 0.5] Zoom Out
  (:`Pressed`
    (`SceneComponent.K2_SetRelativeLocation` (`self.SceneCaptureComponent2D`) (`KismetMathLibrary.MakeVector` (`KismetMathLibrary.FClamp` (- _relativelocation_x 20.0) -400.0 -160.0) _relativelocation_y _relativelocation_z) false false)))

(fn `CreateInspectView`
  (params (InspectInfo :type "/Game/Interaction/Inspect/S_InspectInfo Structure"))
  (bind _returnvalue (`|CreateWidget` "/Game/UserInterface/Inspect/WB_InspectView.WB_InspectView_C" null InspectInfo))
  (bind _output_get (set `self.WB_InspectView` _returnvalue))
  (`UserWidget.AddToViewport` _output_get 0))

(fn `LookAt`
  (returns (Message :type Text))
  (return ""))

(fn `UserConstructionScript`)

(fn `ZoomInFade`
  (bind _wb_inspectview (`self.WB_InspectView`))
  (bind _wb_inspectview_2 (`self.WB_InspectView`))
  (`UserWidget.PlayAnimation` _wb_inspectview_2 (`/Game/UserInterface/Inspect/WB_InspectView.Fade` _wb_inspectview_2) 0.0 1 "Forward" 1.0 false)
  (`UserWidget.PlayAnimation` _wb_inspectview (`/Game/UserInterface/Inspect/WB_InspectView.Enlarge` _wb_inspectview) 0.0 1 "Forward" 1.0 false))

(fn `ZoomOutFade`
  (bind _wb_inspectview (`self.WB_InspectView`))
  (bind _wb_inspectview_2 (`self.WB_InspectView`))
  (`UserWidget.PlayAnimation` _wb_inspectview_2 (`/Game/UserInterface/Inspect/WB_InspectView.Fade` _wb_inspectview_2) 0.0 1 "Reverse" 1.0 false)
  (`UserWidget.PlayAnimation` _wb_inspectview (`/Game/UserInterface/Inspect/WB_InspectView.Enlarge` _wb_inspectview) 0.0 1 "Reverse" 1.0 false))